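; Game mode that builds the initial scenery of the Gameplay level from chained Cidade (city) segments.
; On BeginPlay it checks the level name and calls AddCenário a fixed number of times.
; Each call spawns a Cidade at NextSpawnPoint, then stores that actor's attach transform as the next spawn point, so the segments join end to end.
; An unconnected cast to bairro remains unused.
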(event `self.ReceiveBeginPlay`
  (bind _returnvalue (`GameplayStatics.GetCurrentLevelName` true))
  (if (`KismetStringLibrary.EqualEqual_StrStr` _returnvalue "Gameplay")
    (for _ (range 4)
      (`self.Add Cenário`))))

(event `self.ReceiveTick`
  (params (DeltaSeconds :type "Float (single-precision)")))

(fn `Add Cenário`
  (bind _returnvalue (`|SpawnActorFromClass` "/Game/BP/Cidade.Cidade_C" (`self.NextSpawnPoint`) "Undefined" "OverrideRootScale"))
  (bind _ascidade (cast `/Game/BP/Cidade` _returnvalue))
  (bind _attachtransform (`/Game/BP/Cidade.GetAttachTransform` _ascidade))
  (set `self.NextSpawnPoint` _attachtransform))

(fn `UserConstructionScript`)