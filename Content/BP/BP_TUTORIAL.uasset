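; BP_TUTORIAL is an actor Blueprint, apparently a tutorial exercise, that rotates its root component every frame.
; Tick compares the root's world rotation to a fixed target and, while they differ, rebuilds it from the forward vector plus a constant offset.
; The step ignores delta time and is not directed at the target, so it is frame-rate dependent and not guaranteed to stop there.
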(event `self.ReceiveBeginPlay`)

(event `self.ReceiveTick`
  (params (DeltaSeconds :type "Float (single-precision)"))
  (if (!= (`SceneComponent.K2_GetComponentRotation` (`self.DefaultSceneRoot`)) (struct :`Yaw` 159.0))
    (`SceneComponent.K2_SetWorldRotation` (`self.DefaultSceneRoot`) (`KismetMathLibrary.Conv_VectorToRotator` (+ (`KismetMathLibrary.Conv_RotatorToVector` (`SceneComponent.K2_GetComponentRotation` (`self.DefaultSceneRoot`))) 0.1)) false false)))

(fn `UserConstructionScript`)